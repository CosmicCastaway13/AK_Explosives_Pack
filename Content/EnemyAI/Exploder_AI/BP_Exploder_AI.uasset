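; BP_Exploder_AI is the AI controller for the Exploder enemy.
; On BeginPlay it runs BT_Exploder_Tree, casts the controlled pawn to BP_Exploder_Enemy, and seeds the blackboard with patrol looping and wait time from the pawn's PatrolPath, plus an initial direction.
; The perception update event is empty; the node that would write ME_CanSeePlayer is disconnected, so this controller never updates player sight.
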(event `self.ReceiveBeginPlay`
  (bind _returnvalue (`AIBlueprintHelperLibrary.GetBlackboard` null))
  ;[1 1 1] Runs Behavior Tree
  (`self.RunBehaviorTree` "/Game/EnemyAI/Exploder_AI/BT_Exploder_Tree.BT_Exploder_Tree")
  ;[1 1 1] Sets Patrol Looping
  (bind _asbp_exploder_enemy (cast `/Game/EnemyAI/Exploder_AI/BP_Exploder_Enemy` (`self.K2_GetPawn`)))
  (bind _output_get (set `self.MyPawn` _asbp_exploder_enemy))
  (`BlackboardComponent.SetValueAsBool` (`AIBlueprintHelperLibrary.GetBlackboard` null) "ME_PathLooping" (`/Game/EnemyAI/Exploder_AI/Exploder_Patrol_Path.IsLooping` (`/Game/EnemyAI/Exploder_AI/BP_Exploder_Enemy.Patrol Path` _output_get)))
  ;[1 1 1] Initializes Direction
  (`BlackboardComponent.SetValueAsInt` _returnvalue "ME_Direction" 1)
  ;[1 1 1] Sets Wait Time
  (`BlackboardComponent.SetValueAsFloat` _returnvalue "ME_WaitTime" (`/Game/EnemyAI/Exploder_AI/Exploder_Patrol_Path.WaitTime` (`/Game/EnemyAI/Exploder_AI/BP_Exploder_Enemy.Patrol Path` (`self.MyPawn`)))))

(event `self.AIPerception.OnTargetPerceptionUpdated`
  (params (Actor :type "Actor Object Reference") (Stimulus :type "AIStimulus Structure"))
  ;[1 1 1] Checks To See If Player Is Seen By NPC AI
)

(fn `UserConstructionScript`)